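; Quartz music director that runs the level's beat clock and switches adaptive music stages in time with it.
; BeginPlay creates and starts LevelClock at the set BPM, subscribes to quantization events, and calls InitClock on every BP_QuartzBase actor.
; EnterStage queues a stage, applied on the next Beat or 1/32 event by firing MetaSound start/end triggers on Audio.
; EnterBrige switches to bridge triggers immediately; the beep metronome playback is disconnected.
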(event `self.ReceiveBeginPlay`
  (`self.StarttClock`))

(event `StarttClock`
  (`|ExecutionSequence`
    (:`then_0`
      (bind _returnvalue (`QuartzSubsystem.CreateNewClock` (subsystem `QuartzSubsystem`) "LevelClock" (make `QuartzClockSettings` (make `QuartzTimeSignature` 4)) false true))
      (bind _output_get (set `self.ClockHandle` _returnvalue))
      (`QuartzClockHandle.SetBeatsPerMinute` :`self` _output_get :`QuantizationBoundary` (make `QuartzQuantizationBoundary` "Beat" 2.0) :`BeatsPerMinute` (`self.BPM`)))
    (:`then_1`
      (bind _returnvalue_2 (`GameplayStatics.CreateSound2D` "/Game/Dynamic/MSS/MSS_BeepA4.MSS_BeepA4" 1.0 1.0 0.0 null))
      (bind _output_get_2 (set `self.BeepA4` _returnvalue_2))
      (set `AudioComponent.bCanPlayMultipleInstances` true _output_get_2)
      (bind _returnvalue_3 (`GameplayStatics.CreateSound2D` "/Game/Dynamic/MSS/MSS_BeepA3.MSS_BeepA3" 1.0 1.0 0.0 null))
      (bind _output_get_3 (set `self.BeepA3` _returnvalue_3))
      (set `AudioComponent.bCanPlayMultipleInstances` true _output_get_3))
    (:`then_2`
      (bind _clockhandle (`QuartzClockHandle.StartClock` (`self.ClockHandle`)))
      (`QuartzClockHandle.SubscribeToAllQuantizationEvents` _clockhandle (`|CreateDelegate` :!event `OnQuantizationEvent`)))
    (:`then_3`
      (bind _outactors (`GameplayStatics.GetAllActorsOfClass` "/Game/Dynamic/WTQ_BluePrints/BP_QuartzBase.BP_QuartzBase_C"))
      (for _array_element _outactors
        (`/Game/Dynamic/WTQ_BluePrints/BP_QuartzBase.InitClock` _array_element)))))

(event `OnQuantizationEvent`
  (params (ClockName :type Name) (QuantizationType :type "EQuartzCommandQuantization Enum" :default "Bar") (NumBars :type Integer) (Beat :type Integer) (BeatFraction :type "Float (single-precision)"))
  (bind _newstage (`self.NewStage`))
  ;[0.15 0 0 0.5] OnQuantizationEvent
  (switch `EQuartzCommandQuantization` QuantizationType
    (:`Beat`
      _)
    (:`ThirtySecondNote`
      _))
  (if (not (== (`self.NewStage`) (`self.Stage`)))
    (`self.SwitchOnBeat` _newstage)
    (set `self.Stage` _newstage)
    (`KismetSystemLibrary.PrintString` "Stage Switch")))

(event `EnterStage`
  (params (stage :type Integer))
  ; Stage Switch
  (set `self.NewStage` stage))

(event `SwitchOnBeat`
  (params (Selection :type Integer))
  (bind _audio (`self.Audio`))
  ; Stage Switch
  (`AudioComponent.SetSound` (`self.Audio`) "/Game/Dynamic/MSS/MSS_Stage.MSS_Stage")
  (switch `int` Selection
    (:`0`
      (`AudioParameterControllerInterface.SetTriggerParameter` _audio "StageFinal")
      (`AudioParameterControllerInterface.SetTriggerParameter` _audio "Stage5End"))
    (:`1`
      (`AudioParameterControllerInterface.SetTriggerParameter` _audio "Stage1")
      (`AudioParameterControllerInterface.SetTriggerParameter` _audio "Stage2End"))
    (:`2`
      (`AudioParameterControllerInterface.SetTriggerParameter` _audio "Stage2")
      (`AudioParameterControllerInterface.SetTriggerParameter` _audio "Stage1End")
      (`AudioParameterControllerInterface.SetTriggerParameter` _audio "Stage3End"))
    (:`3`
      (`AudioParameterControllerInterface.SetTriggerParameter` _audio "Stage3")
      (`AudioParameterControllerInterface.SetTriggerParameter` _audio "Stage2End")
      (`AudioParameterControllerInterface.SetTriggerParameter` _audio "Stage4End"))
    (:`4`
      (`AudioParameterControllerInterface.SetTriggerParameter` _audio "Stage4")
      (`AudioParameterControllerInterface.SetTriggerParameter` _audio "Stage3End")
      (`AudioParameterControllerInterface.SetTriggerParameter` _audio "Stage5End"))
    (:`5`
      (`AudioParameterControllerInterface.SetTriggerParameter` _audio "Stage5")
      (`AudioParameterControllerInterface.SetTriggerParameter` _audio "Stage4End"))))

(event `EnterBrige`
  (params (Selection :type Integer))
  (bind _audio (`self.Audio`))
  (`AudioComponent.SetSound` (`self.Audio`) "/Game/Dynamic/MSS/MSS_Bridge.MSS_Bridge")
  (switch `int` Selection
    (:`0`
      (`AudioParameterControllerInterface.SetTriggerParameter` _audio "Bridge1" :!label _label))
    (:`1`
      (goto _label))
    (:`2`
      (`AudioParameterControllerInterface.SetTriggerParameter` _audio "Bridge2"))
    (:`3`
      (`AudioParameterControllerInterface.SetTriggerParameter` _audio "Bridge3"))
    (:`4`
      (`AudioParameterControllerInterface.SetTriggerParameter` _audio "Bridge4"))))

(fn `UserConstructionScript`)