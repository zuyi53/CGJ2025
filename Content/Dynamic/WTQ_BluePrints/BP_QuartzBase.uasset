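; BP_QuartzBase is a base Blueprint for objects that react to the beat of a Quartz music clock.
; InitClock fetches the "LevelClock" handle from the Quartz subsystem, subscribes to all its quantization events and stores the handle.
; Each event calls OnBeatTick, which is empty here, then CheckBeatChange compares the beat with CurBeat.
; OnBeatChange fires only when the beat differs and by default prints the object's name.
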(event `InitClock`
  (`self.On Init Clock`))

(event `CustomEvent`
  (params (ClockName :type Name) (QuantizationType :type "EQuartzCommandQuantization Enum" :default "Bar") (NumBars :type Integer) (Beat :type Integer) (BeatFraction :type "Float (single-precision)"))
  (`self.On Beat Tick` Beat BeatFraction)
  (`self.Check Beat Change` Beat))

(fn `Check Beat Change`
  (params (InputPin :type Integer))
  (if (not (== InputPin (`self.CurBeat`)))
    (bind _output_get (set `self.CurBeat` InputPin))
    (`self.On Beat Change` _output_get)))

(fn `On Beat Change`
  (params (NewBeat :type Integer))
  (`KismetSystemLibrary.PrintString` (`KismetSystemLibrary.GetDisplayName` self)))

(fn `On Beat Tick`
  (params (Beat :type Integer) (BeatFraction :type "Float (double-precision)")))

(fn `On Init Clock`
  (bind _returnvalue (`QuartzSubsystem.GetHandleForClock` (subsystem `QuartzSubsystem`) "LevelClock"))
  (bind _clockhandle (`QuartzClockHandle.SubscribeToAllQuantizationEvents` _returnvalue (`|CreateDelegate` :!event `CustomEvent`)))
  (set `self.Clock Handle` _clockhandle))

(fn `UserConstructionScript`)