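; BP_QuartzCube_Fade is a beat-driven cube that alternates between solid and absent, likely synced to Quartz as its name suggests.
; It overrides the parent's On Beat Change, calls the parent logic, then uses the FlipFlop boolean to toggle both visibility and collision on the Cube.
; Despite the Fade name, the switch is instant, with no opacity blend in this graph.
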(fn `On Beat Change`
  (params (NewBeat :type Integer))
  (bind _flipflop (`self.FlipFlop`))
  (bind _cube (`self.Cube`))
  (bind _cube_2 (`self.Cube`))
  (`parent.On Beat Change` NewBeat)
  (if (`self.FlipFlop`)
    (`SceneComponent.SetVisibility` _cube_2 _flipflop false)
    (`PrimitiveComponent.SetCollisionEnabled` _cube_2 "QueryAndPhysics")
    (set `self.FlipFlop` (not (`self.FlipFlop`)))
    (else
      (`SceneComponent.SetVisibility` _cube _flipflop false)
      (`PrimitiveComponent.SetCollisionEnabled` _cube "NoCollision")
      (set `self.FlipFlop` (not (`self.FlipFlop`))))))

(fn `UserConstructionScript`
  (`parent.UserConstructionScript`))