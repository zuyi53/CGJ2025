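; BP_QuartzCube_Rotate is a cube that swings between two rotations in time with the beat callbacks of its parent class.
; OnBeatTick converts the beat fraction into an alpha and lerps the Cube's world rotation between Rot01 and Rot02.
; OnBeatChange toggles FlipFlop to reverse the lerp direction each beat; an unconnected visibility toggle remains there.
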(fn `On Beat Change`
  (params (NewBeat :type Integer))
  (`parent.On Beat Change` NewBeat)
  (set `self.FlipFlop` (not (`self.FlipFlop`))))

(fn `On Beat Tick`
  (params (Beat :type Integer) (BeatFraction :type "Float (double-precision)"))
  (`parent.On Beat Tick` Beat BeatFraction)
  (bind _newparam (`self.ConvertFraction` BeatFraction))
  (if (`self.FlipFlop`)
    (`SceneComponent.K2_SetWorldRotation` (`self.Cube`) (`KismetMathLibrary.RLerp` (`self.Rot01`) (`self.Rot02`) _newparam) false false)
    (else
      (`SceneComponent.K2_SetWorldRotation` (`self.Cube`) (`KismetMathLibrary.RLerp` (`self.Rot02`) (`self.Rot01`) _newparam) false false))))

(fn `On Init Clock`
  (`parent.On Init Clock`))

(fn `UserConstructionScript`
  (`parent.UserConstructionScript`))