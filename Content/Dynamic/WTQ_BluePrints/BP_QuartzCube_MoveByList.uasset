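; Quartz beat-synced cube that moves along a looping list of offset positions, one segment per beat.
; On clock init it caches the root's world location as the origin for the PosList offsets.
; Each beat tick lerps the Cube between the current and next point using the converted beat fraction.
; Each beat change advances the index, wrapping back to the first point.
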(fn `On Beat Change`
  (params (NewBeat :type Integer))
  (bind _returnvalue (+ (`self.CurIndex`) 1))
  (`parent.On Beat Change` NewBeat)
  (if (>= _returnvalue (`KismetArrayLibrary.Array_Length` (`self.PosList`)))
    (set `self.CurIndex` 0)
    (else
      (set `self.CurIndex` _returnvalue))))

(fn `On Beat Tick`
  (params (Beat :type Integer) (BeatFraction :type "Float (double-precision)"))
  (`parent.On Beat Tick` Beat BeatFraction)
  (bind _newparam (`self.ConvertFraction` BeatFraction))
  (if (> (`KismetArrayLibrary.Array_Length` (`self.PosList`)) (+ (`self.CurIndex`) 1))
    (`SceneComponent.K2_SetWorldLocation` (`self.Cube`) (+ (`KismetMathLibrary.VLerp` (`|GetArrayItem` (`self.PosList`) (`self.CurIndex`)) (`|GetArrayItem` (`self.PosList`) (+ (`self.CurIndex`) 1)) _newparam) (`self.SelfLocation`)) false false)
    (else
      (`SceneComponent.K2_SetWorldLocation` (`self.Cube`) (+ (`KismetMathLibrary.VLerp` (`|GetArrayItem` (`self.PosList`) (`self.CurIndex`)) (`|GetArrayItem` (`self.PosList`)) _newparam) (`self.SelfLocation`)) false false))))

(fn `On Init Clock`
  (`parent.On Init Clock`)
  (set `self.SelfLocation` (`SceneComponent.K2_GetComponentLocation` (`self.DefaultSceneRoot`))))

(fn `UserConstructionScript`
  (`parent.UserConstructionScript`))