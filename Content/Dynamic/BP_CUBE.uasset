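; BP_CUBE is an audio visualizer actor that pulses two cylinders with the loudness of a sound.
; Construction assigns the LoudnessAnalyzer's sound to the Audio component and caches its duration.
; On BeginPlay it plays the audio, and each playback-percent update converts to seconds to sample normalized precomputed-style loudness per channel.
; Channels 0 and 1 drive the uniform scale of one cylinder each, with channel 0 also printed for debugging.
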(event `self.ReceiveBeginPlay`
  (add `AudioComponent.OnAudioPlaybackPercent` (`self.Audio`) (delegate `PlaybackPercentEvent`))
  (`AudioComponent.Play` (`self.Audio`) 0.0))

(event `PlaybackPercentEvent`
  (params (PlayingSoundWave :type "SoundWave Object Reference") (PlaybackPercent :type "Float (single-precision)"))
  (bind _loudnessanalyzer (`self.LoudnessAnalyzer`))
  (bind _returnvalue (* PlaybackPercent (`self.Duration`)))
  (bind _outloudness (`LoudnessNRT.GetNormalizedChannelLoudnessAtTime` _loudnessanalyzer _returnvalue 0))
  (`KismetSystemLibrary.PrintString` (`KismetStringLibrary.Conv_DoubleToString` _outloudness))
  (`SceneComponent.SetRelativeScale3D` (`self.Cylinder`) (`KismetMathLibrary.Conv_DoubleToVector` (* _outloudness 3.0)))
  (`SceneComponent.SetRelativeScale3D` (`self.Cylinder1`) (`KismetMathLibrary.Conv_DoubleToVector` (* (`LoudnessNRT.GetNormalizedChannelLoudnessAtTime` _loudnessanalyzer _returnvalue 1) 3.0))))

(fn `UserConstructionScript`
  (bind _sound (`AudioAnalyzerNRT.Sound` (`self.LoudnessAnalyzer`)))
  (`AudioComponent.SetSound` (`self.Audio`) _sound)
  (set `self.Duration` (`SoundBase.Duration` _sound)))