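; Music-reactive floor piece whose cube changes height with the loudness of the music played by BP_QurtzCore.
; On BeginPlay it takes the first BP_QurtzCore in the level, binds to its audio playback-percent event and caches the sound's duration.
; Each playback update converts percent to seconds, samples the precomputed LoudnessAnalyzer's normalized channel loudness at that time, and applies it as the cube's Z scale.
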(event `self.ReceiveBeginPlay`
  (bind _outactors (`GameplayStatics.GetAllActorsOfClass` "/Game/Dynamic/BP_QurtzCore.BP_QurtzCore_C"))
  (bind _output_get (set `self.QurtzRef` (`|GetArrayItem` _outactors)))
  (bind _audio (`/Game/Dynamic/BP_QurtzCore.Audio` _output_get))
  (add `AudioComponent.OnAudioPlaybackPercent` _audio (delegate `PlaybackPercentEvent`))
  (set `self.Duration` (`SoundBase.Duration` (`AudioComponent.Sound` _audio))))

(event `PlaybackPercentEvent`
  (params (PlayingSoundWave :type "SoundWave Object Reference") (PlaybackPercent :type "Float (single-precision)"))
  (`SceneComponent.SetRelativeScale3D` (`self.Cube`) (`KismetMathLibrary.MakeVector` 1.0 1.0 (* (`LoudnessNRT.GetNormalizedChannelLoudnessAtTime` (`self.LoudnessAnalyzer`) (* PlaybackPercent (`self.Duration`)) 0) 1.0))))

(fn `UserConstructionScript`)