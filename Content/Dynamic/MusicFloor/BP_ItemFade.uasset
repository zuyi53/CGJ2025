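; BP_ItemFade is an audio-reactive music floor item that scales its skeletal mesh with the loudness of the music.
; On BeginPlay it finds the first BP_QurtzCore, binds to its audio playback-percent event and caches the sound's duration.
; Each update converts percent to seconds, samples precomputed normalized channel-zero loudness from LoudnessAnalyzer, and applies it, multiplied up, as uniform relative scale.
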(event `self.ReceiveBeginPlay`
  (`parent.ReceiveBeginPlay`)
  (bind _outactors (`GameplayStatics.GetAllActorsOfClass` "/Game/Dynamic/BP_QurtzCore.BP_QurtzCore_C"))
  (bind _output_get (set `self.QurtzRef` (`|GetArrayItem` _outactors)))
  (bind _audio (`/Game/Dynamic/BP_QurtzCore.Audio` _output_get))
  (add `AudioComponent.OnAudioPlaybackPercent` _audio (delegate `PlaybackPercentEvent`))
  (set `self.Duration` (`SoundBase.Duration` (`AudioComponent.Sound` _audio))))

(event `PlaybackPercentEvent`
  (params (PlayingSoundWave :type "SoundWave Object Reference") (PlaybackPercent :type "Float (single-precision)"))
  (bind _returnvalue (* (`LoudnessNRT.GetNormalizedChannelLoudnessAtTime` (`self.LoudnessAnalyzer`) (* PlaybackPercent (`self.Duration`)) 0) 10.0))
  (`SceneComponent.SetRelativeScale3D` (`self.SkeletalMesh`) (`KismetMathLibrary.MakeVector` _returnvalue _returnvalue _returnvalue)))

(fn `UserConstructionScript`
  (`parent.UserConstructionScript`))